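; BP_TV is a TV Blueprint that plays a video and publishes its playback progress to materials.
; On BeginPlay it opens the TV file media source on a Media Player and starts playback.
; While playing, each Tick writes normalized playback time to the Alpha scalar in the MPC_TV parameter collection, so materials reading it can stay in sync with the video.
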(event `self.ReceiveBeginPlay`
  (bind _mediaplayer (`self.MediaPlayer`))
  (`MediaPlayer.OpenSource` _mediaplayer "/Game/TVLight/TV_FileMediaSource.TV_FileMediaSource")
  (`MediaPlayer.Play` _mediaplayer))

(event `self.ReceiveTick`
  (params (DeltaSeconds :type "Float (single-precision)"))
  (bind _mediaplayer (`self.MediaPlayer`))
  (if (`MediaPlayer.IsPlaying` _mediaplayer)
    (`KismetMaterialLibrary.SetScalarParameterValue` "/Game/TVLight/MPC_TV.MPC_TV" "Alpha" (/ (`KismetMathLibrary.GetTotalSeconds` (`MediaPlayer.GetTime` _mediaplayer)) (`KismetMathLibrary.GetTotalSeconds` (`MediaPlayer.GetDuration` _mediaplayer))))))

(fn `UserConstructionScript`)